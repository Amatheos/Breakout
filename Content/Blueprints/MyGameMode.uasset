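; Game mode for a block-breaking ball game, managing score, lives and game state.
; On BeginPlay it creates the Interface widget and calls PlayAgain, which reloads the LevelBlocks streaming level to restore blocks, resets score and lives, and calls ResetPlayerPosition and StartGame.
; UpdateScore clamps the score at zero and pushes it to the widget.
; BallDropped decrements and displays lives, or switches to the game-over state when none remain.
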(event `self.ReceiveBeginPlay`
  ;[1 1 1] Create widget and launch the game
  (bind _returnvalue (`|CreateWidget` "/Game/Blueprints/Interface.Interface_C"))
  (bind _output_get (set `self.Interface` _returnvalue))
  (`UserWidget.AddToViewport` _output_get 0)
  (`self.Play again`))

(event `Play again`
  (bind _max_lives (`self.Max lives`))
  (bind _interface (`self.Interface`))
  ;[1 1 1] Restart game
  (`self.Load blocks`)
  (set `self.Lives left` _max_lives)
  (set `/Game/Blueprints/Interface.Lives left` _max_lives _interface)
  (set `/Game/Blueprints/Interface.Score` 0 _interface)
  (set `self.Score` 0)
  (`self.ResetPlayerPosition`)
  (set `self.CurrentGameState` "NewEnumerator0")
  (`self.StartGame`))

(event `Load blocks`
  ;[1 1 1] Reaload destroyed blocks
  (`GameplayStatics.UnloadStreamLevel` "LevelBlocks")
  (`GameplayStatics.LoadStreamLevel` "LevelBlocks" true))

(event `Update score`
  (params (Score :type Integer))
  (bind _returnvalue (+ Score (`self.Score`)))
  ;[1 1 1] Update score
  (if (< _returnvalue 0)
    (set `self.Score` 0)
    (else
      (set `self.Score` _returnvalue)))
  (set `/Game/Blueprints/Interface.Score` (`self.Score`) (`self.Interface`)))

(event `Ball dropped`
  (bind _lives_left (`self.Lives left`))
  ;[1 1 1] Spawn new ball and decrement lives
  (if (<= _lives_left 0)
    (`self.Game over`)
    (else
      (bind _output_get (set `self.Lives left` (- _lives_left 1)))
      (set `/Game/Blueprints/Interface.Lives left` _output_get (`self.Interface`)))))

(event `Game over`
  ;[1 1 1] Change game state when it is over
  (set `self.CurrentGameState` "NewEnumerator1"))

(fn `UserConstructionScript`)