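; Ball actor that follows the player's Arrow component until launched by a physics impulse, then bounces around at constant speed.
; Each tick it forces velocity to Speed and snaps its yaw to the nearest horizontal diagonal by rotating 45 degrees, rounding to 90 and rotating back.
; Hits play audio, and destruction notifies MyGameMode of the drop and has the Player spawn a replacement.
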(event Custom|Update%20position
  ;[1 1 1] Update ball position
  (if (not (Variables|Default|GetActive))
    (Transformation|SetActorLocation (Transformation|GetWorldLocation (Variables|/Game/Blueprints/Player.Player_C|GetArrow (Variables|Default|GetPlayer))) false false)))

(event Custom|Launch
  (params (Direction :type Vector))
  ;[1 1 1] Add impulse to launch the ball
  (Variables|Default|SetActive true)
  (Physics|AddImpulse (Variables|Default|GetBall) Direction "None" true))

(event Custom|Clamp%20Velocity
  (bind _returnvalue (Transformation|GetVelocity))
  (bind _returnvalue_2 (Math|Rotator|MakeRotator 0.0 0.0 45.0))
  (bind _speed (Variables|Default|GetSpeed))
  (bind _returnvalue_3 (Math|Vector|ClampVectorSize _returnvalue _speed _speed))
  ;[1 1 1] Make sure, ball always bounces on 45 degrees
  (Physics|SetPhysicsLinearVelocity (Variables|Default|GetBall) (* (Math|Vector|UnrotateVector (Math|Rotator|GetRotationXVector (Math|Rotator|MakeRotator 0.0 0.0 (|((round((A/B)))*B) (.yaw (Math|Rotator|MakeRotfromX (Math|Vector|RotateVector _returnvalue_3 _returnvalue_2))) 9e+01))) _returnvalue_2) (Math|Vector|VectorLength _returnvalue_3)) false "None"))

(event EventBeginPlay
  ;[1 1 1] Get player and set game mode
  (bind _asplayer (Utilities|Casting|CastToPlayer (Pawn|GetControlledPawn (Game|GetPlayerController 0))))
  (Variables|Default|SetPlayer _asplayer)
  (bind _asmy_game_mode (Utilities|Casting|CastToMyGameMode (Game|GetGameMode)))
  (Variables|Default|SetGame%20mode _asmy_game_mode))

(event Collision|EventHit
  (params (MyComp :type Primitive%20Component%20Object%20Reference) (Other :type Actor%20Object%20Reference) (OtherComp :type Primitive%20Component%20Object%20Reference) (bSelfMoved :type Boolean) (HitLocation :type Vector :default "0, 0, 0") (HitNormal :type Vector :default "0, 0, 0") (NormalImpulse :type Vector :default "0, 0, 0") (Hit :type Hit%20Result%20Structure%20%28by%20ref%29))
  ;[1 1 1] Play audio when ball hits anything
  (Audio|Components|Audio|Play (Variables|Default|GetAudio) 0.0))

(event EventTick
  (params (DeltaSeconds :type Float%20%28single-precision%29))
  ;[1 1 1] Move ball each frame
  (CallFunction|UpdatePosition)
  (CallFunction|ClampVelocity))

(event EventDestroyed
  ;[1 1 1] Spawn a new ball when old one is destroyed
  (Default|BallDropped (Variables|Default|GetGame%20mode))
  (Default|SpawnBall (Variables|Default|GetPlayer)))

(fn ConstructionScript)