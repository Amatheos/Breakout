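; Player Blueprint for a paddle-and-ball game, handling paddle movement, ball launching and game controls.
; Horizontal axis input pushes the paddle along X with physics impulses scaled by Speed.
; BeginPlay spawns a Ball at the Arrow component's transform, and Fire launches it along the arrow's forward vector if it is valid and not yet active.
; Separate inputs restart by reopening the current level or quit the game.
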(event `InputAxis|MoveHorizontally`
  (params (AxisValue :type "Float (single-precision)"))
  ;[1 1 1] Move paddle
  (`PrimitiveComponent.AddImpulse` (`self.Paddle`) (`KismetMathLibrary.MakeVector` (* AxisValue (`self.Speed`))) "None" false))

(event `self.ReceiveBeginPlay`
  ;[1 1 1] Spawn ball at the start of the game
  (`self.Spawn Ball`))

(event `Spawn Ball`
  ;[1 1 1] Spawn ball at certain position
  (bind _returnvalue (`|SpawnActorFromClass` "/Game/Blueprints/Ball.Ball_C" (`SceneComponent.K2_GetComponentToWorld` (`self.Arrow`)) "AlwaysSpawn" "OverrideRootScale" null null))
  (set `self.Ball` _returnvalue))

(event `InputAction|Fire`
  (params (Key :type "Key Structure"))
  (bind _ball (`self.Ball`))
  ;[1 1 1] Launch ball
  (:`Pressed`
    (if (and (`KismetSystemLibrary.IsValid` _ball) (not (`/Game/Blueprints/Ball.Active` _ball)))
      (`/Game/Blueprints/Ball.Launch` _ball (`KismetMathLibrary.Conv_RotatorToVector` (`SceneComponent.K2_GetComponentRotation` (`self.Arrow`)))))))

(event `InputAction|Reset game`
  (params (Key :type "Key Structure"))
  ;[1 1 1] Restart game on spacebar
  (:`Pressed`
    (bind _returnvalue (`GameplayStatics.GetCurrentLevelName` true))
    (`GameplayStatics.OpenLevel` (`KismetStringLibrary.Conv_StringToName` _returnvalue))))

(event `InputAction|Quit`
  (params (Key :type "Key Structure"))
  ;[1 1 1] Quit on esc pressed
  (:`Pressed`
    (`KismetSystemLibrary.QuitGame` null "Quit")))

(fn `UserConstructionScript`)